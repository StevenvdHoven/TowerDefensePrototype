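; BP_Player is the prototype player character with melee combo attacks, health, and a meditation form.
; On BeginPlay it spawns a BP_MeditateState pawn that it possesses on Meditate and forwards quick summon and recall to.
; Attacks cycle montages using Tick-driven cooldown and combo timers, damaging I_Damageable characters via a forward sphere overlap.
; Damage and spirit-cost events refresh the HUD's health and spirit bars, and death opens the menu level.
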(event Custom|SpiritCost
  (CallFunction|UpdateUI))

(event Input|EnhancedActionEvents|EnhancedInputActionIA_Meditate
  (params (ActionValue :type Boolean) (ElapsedSeconds :type Float%20%28double-precision%29) (TriggeredSeconds :type Float%20%28double-precision%29) (InputAction :type Input%20Action%20Object%20Reference :default "/Game/PROTOTYE/Input/IA_Meditate.IA_Meditate"))
  (Pawn|Possess (Pawn|GetController) (Variables|Default|GetMeditatePawn)))

(event Input|EnhancedActionEvents|EnhancedInputActionIA_Attack
  (params (ActionValue :type Boolean) (ElapsedSeconds :type Float%20%28double-precision%29) (TriggeredSeconds :type Float%20%28double-precision%29) (InputAction :type Input%20Action%20Object%20Reference :default "/Game/PROTOTYE/Input/IA_Attack.IA_Attack"))
  (CallFunction|Attack))

(event Input|EnhancedActionEvents|EnhancedInputActionIA_QuickSummon
  (params (ActionValue :type Boolean) (ElapsedSeconds :type Float%20%28double-precision%29) (TriggeredSeconds :type Float%20%28double-precision%29) (InputAction :type Input%20Action%20Object%20Reference :default "/Game/PROTOTYE/Input/IA_QuickSummon.IA_QuickSummon"))
  (Default|QuickSummon (Variables|Default|GetMeditatePawn)))

(event Input|EnhancedActionEvents|EnhancedInputActionIA_Recall
  (params (ActionValue :type Boolean) (ElapsedSeconds :type Float%20%28double-precision%29) (TriggeredSeconds :type Float%20%28double-precision%29) (InputAction :type Input%20Action%20Object%20Reference :default "/Game/PROTOTYE/Input/IA_Recall.IA_Recall"))
  (Default|Recall (Variables|Default|GetMeditatePawn)))

(event EventTick
  (params (DeltaSeconds :type Float%20%28single-precision%29))
  (Utilities|FlowControl|Sequence
    (:then_0
      (if (> (Variables|Attack|GetAttackIndex) 0)
        (bind _output_get (Variables|Attack|SetComboTimer (- (Variables|Attack|GetComboTimer) DeltaSeconds)))
        (if (< _output_get 0.0)
          (Variables|Attack|SetAttackIndex 0))))
    (:then_1
      (if (> (Variables|Attack|GetAttackTimer) 0.0)
        (Variables|Attack|SetAttackTimer (- (Variables|Attack|GetAttackTimer) DeltaSeconds))))))

(event EventBeginPlay
  (bind _returnvalue (Game|GetPlayerController 0))
  (Input|SetInputModeGameOnly _returnvalue false)
  (Variables|/Script/Engine.PlayerController|SetbShowMouseCursor _returnvalue false)
  (Input|AddMappingContext (PlayerController|LocalPlayerSubsystems|GetEnhancedInputLocalPlayerSubsystem _returnvalue) "/Game/PROTOTYE/Input/IMC_PrototypeInputMap.IMC_PrototypeInputMap" 0 "(bIgnoreAllPressedKeysUntilRelease=True,bForceImmediately=False,bNotifyUserSettings=False)")
  (bind _returnvalue_2 (Game|SpawnActorfromClass "/Game/PROTOTYE/Player/BP_MeditateState.BP_MeditateState_C" (Math|Transform|MakeTransform (Transformation|GetActorLocation)) "AlwaysSpawn" "MultiplyWithRoot" 0 0))
  (bind _output_get (Variables|Default|SetMeditatePawn _returnvalue_2))
  (Utilities|FlowControl|Sequence
    (:then_0
      (bind _returnvalue_3 (UserInterface|CreateWidget "/Game/PROTOTYE/Player/WBP_PlayerHUD.WBP_PlayerHUD_C"))
      (bind _output_get_2 (Variables|Default|SetUI _returnvalue_3))
      (UserInterface|Viewport|AddtoViewport _output_get_2 0))
    (:then_1
      (EventDispatchers|BindEventtoOnSpiritCost _output_get (delegate Custom|SpiritCost)))))

(event EventTakeDamage
  (params (Damage :type Integer))
  (bind _output_get (Variables|Default|SetHealth (Math|Integer|Clamp(Integer) (- (Variables|Default|GetHealth) Damage) 0 100)))
  (CallFunction|UpdateUI)
  (if (<= _output_get 0)
    (Game|OpenLevel(byObjectReference) "/Game/PROTOTYE/Menu/L_Menu.L_Menu")))

(fn ConstructionScript
  (|CallParentFunction))

(fn Attack
  (bind _returnvalue (Math|Float|MakeLiteralFloat 1e+02))
  (bind _returnvalue_2 (Transformation|GetActorLocation))
  (bind _returnvalue_3 (Transformation|GetActorForwardVector))
  (bind _attackmontages (Variables|Attack|GetAttackMontages))
  (bind _returnvalue_4 (* _returnvalue_3 1e+02))
  (bind _returnvalue_5 (+ _returnvalue_2 _returnvalue_4))
  (if (<= (Variables|Attack|GetAttackTimer) 0.0)
    (if (Utilities|Array|IsValidIndex _attackmontages)
      (Utilities|FlowControl|Sequence
        (:then_0
          (Animation|Montage|MontagePlay (Components|SkeletalMesh|GetAnimInstance (Variables|Character|GetMesh)) (Utilities|Array|Get(acopy) _attackmontages (Variables|Attack|GetAttackIndex)) 1.0 "MontageLength" 0.0 true)
          (Variables|Attack|SetComboTimer (Variables|Attack|GetComboCooldown)))
        (:then_1
          (Variables|Attack|SetAttackTimer (Variables|Attack|GetAttackCooldown))
          (bind _result (Math|Integer|IncrementInt (Variables|Attack|GetAttackIndex))
            (:%20%20
              (if (> _result (- (Utilities|Array|Length (Variables|Attack|GetAttackMontages)) 1))
                (Variables|Attack|SetAttackIndex 0)))))
        (:then_2
          (bind (_outactors _returnvalue_6) (Collision|SphereOverlapActors _returnvalue_5 _returnvalue (Utilities|Array|MakeArray "ObjectTypeQuery1" "ObjectTypeQuery2" "ObjectTypeQuery3" "ObjectTypeQuery4" "ObjectTypeQuery6") "/Script/Engine.Character" (Utilities|Array|MakeArray self)))
          (Utilities|FlowControl|Sequence
            (:then_0
              (if _returnvalue_6
                (for _array_element _outactors
                  (Utilities|FlowControl|Sequence
                    (:then_0
                      (bind _asi_damageable (Utilities|Casting|CastToI_Damageable _array_element))
                      (Default|TakeDamage _asi_damageable 20))
                    (:then_1
                      (Development|PrintString (Utilities|String|Append (Utilities|String|MakeLiteralString "Attacked - ") (Utilities|GetDisplayName _array_element))))))))
            (:then_1
              (Rendering|Debug|DrawDebugSphere _returnvalue_5 _returnvalue 12 "(R=1.000000,G=0.056630,B=0.000000,A=1.000000)" 1.0))))))))

(fn UpdateUI
  (bind _meditatepawn (Variables|Default|GetMeditatePawn))
  (Utilities|FlowControl|Sequence
    (:then_0
      (Default|SetHealthPercent (Variables|Default|GetUI) (/ (Math|Conversions|ToFloat(Integer) (Variables|Default|GetHealth)) 1e+02)))
    (:then_1
      (Default|SetSpiritEnergy (Variables|Default|GetUI) (/ (Variables|/Game/PROTOTYE/Player/BP_MeditateState.BP_MeditateState_C|GetSpiritEnergy _meditatepawn) (Variables|/Game/PROTOTYE/Player/BP_MeditateState.BP_MeditateState_C|GetMaxSpiritEnergy _meditatepawn))))))