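; BP_MeditateState is the player's meditation pawn, a height-adjustable free camera for summoning an ally spirit.
; While possessed it adds its input mapping, moves and scrolls height, and spawns the spirit at a camera trace hit; meditate input repossesses BP_Player.
; Unpossessed, it hovers above the player.
; It always recharges SpiritEnergy and exposes QuickSummon beside the player and Recall, allowing one spirit at a time.
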(event Input|EnhancedActionEvents|EnhancedInputActionIA_Move
  (params (ActionValue :type Vector%202D%20Structure) (ElapsedSeconds :type Float%20%28double-precision%29) (TriggeredSeconds :type Float%20%28double-precision%29) (InputAction :type Input%20Action%20Object%20Reference :default "/Game/Input/Actions/IA_Move.IA_Move"))
  (bind _returnvalue (Transformation|GetActorLocation))
  (bind _camera (Variables|Default|GetCamera))
  (bind _movementspeed (Variables|Default|GetMovementSpeed))
  (bind _returnvalue_2 (Math|Vector|GetRightVector _camera))
  (bind _returnvalue_3 (Math|Vector|GetForwardVector _camera))
  (bind _returnvalue_4 (* _returnvalue_3 (.y ActionValue)))
  (bind _returnvalue_5 (* _returnvalue_2 (.x ActionValue)))
  (bind _returnvalue_6 (+ _returnvalue_4 _returnvalue_5))
  (bind _returnvalue_7 (Math|Vector|Normalize _returnvalue_6))
  (bind _returnvalue_8 (* _returnvalue_7 _movementspeed))
  (bind _returnvalue_9 (+ _returnvalue _returnvalue_8))
  (if (Class|Pawn|IsControlled)
    (Transformation|SetActorLocation (Math|Vector|MakeVector (.x _returnvalue_9) (.y _returnvalue_9) (Variables|Default|GetHeight)) true false)))

(event Input|EnhancedActionEvents|EnhancedInputActionIA_Meditate
  (params (ActionValue :type Boolean) (ElapsedSeconds :type Float%20%28double-precision%29) (TriggeredSeconds :type Float%20%28double-precision%29) (InputAction :type Input%20Action%20Object%20Reference :default "/Game/PROTOTYE/Input/IA_Meditate.IA_Meditate"))
  (bind _asbp_player (Utilities|Casting|CastToBP_Player (Variables|Default|GetPlayer)))
  (Pawn|Possess (Pawn|GetController) _asbp_player))

(event Input|EnhancedActionEvents|EnhancedInputActionIA_Scroll
  (params (ActionValue :type Float%20%28double-precision%29) (ElapsedSeconds :type Float%20%28double-precision%29) (TriggeredSeconds :type Float%20%28double-precision%29) (InputAction :type Input%20Action%20Object%20Reference :default "/Game/PROTOTYE/Input/IA_Scroll.IA_Scroll"))
  (bind _returnvalue (Transformation|GetActorLocation))
  (Variables|Default|SetHeight (Math|Float|Clamp(Float) (+ (Variables|Default|GetHeight) (* (* ActionValue (Variables|Default|GetScrollSpeed)) -1.0)) (Variables|Default|GetMinHeight) (Variables|Default|GetMaxHeight)))
  (Transformation|SetActorLocation (Math|Vector|MakeVector (.x _returnvalue) (.y _returnvalue) (Variables|Default|GetHeight)) false true))

(event Input|EnhancedActionEvents|EnhancedInputActionIA_Look
  (params (ActionValue :type Vector%202D%20Structure) (ElapsedSeconds :type Float%20%28double-precision%29) (TriggeredSeconds :type Float%20%28double-precision%29) (InputAction :type Input%20Action%20Object%20Reference :default "/Game/HorseStarterKit/Input/Actions/IA_Look.IA_Look"))
  (Pawn|Input|AddControllerPitchInput (.y ActionValue))
  (Pawn|Input|AddControllerYawInput (.x ActionValue)))

(event Input|EnhancedActionEvents|EnhancedInputActionIA_Attack
  (params (ActionValue :type Boolean) (ElapsedSeconds :type Float%20%28double-precision%29) (TriggeredSeconds :type Float%20%28double-precision%29) (InputAction :type Input%20Action%20Object%20Reference :default "/Game/PROTOTYE/Input/IA_Attack.IA_Attack"))
  (bind _returnvalue (Transformation|GetActorLocation))
  (if (Class|Pawn|IsControlled)
    (bind (_outhit _returnvalue_2) (Collision|LineTraceByChannel _returnvalue (+ _returnvalue (* (Math|Vector|GetForwardVector (Variables|Default|GetCamera)) 1e+05)) "TraceTypeQuery1" true 0 "ForDuration" true "(R=1.000000,G=0.000000,B=0.000000,A=1.000000)" "(R=0.000000,G=1.000000,B=0.000000,A=1.000000)" 2.0))
    (if _returnvalue_2
      (Utilities|IsValid (Variables|Default|GetSpawnedSpirit)
        (:Is%20Not%20Valid
          (bind _returnvalue_3 (Game|SpawnActorfromClass "/Game/PROTOTYE/Spirits/BP_AllySpirit.BP_AllySpirit_C" (Math|Transform|MakeTransform (.Location (Collision|BreakHitResult _outhit))) "AlwaysSpawn" "MultiplyWithRoot" 0 0))
          (Variables|Default|SetSpawnedSpirit _returnvalue_3)
          (Variables|Default|SetSpiritEnergy (Math|Float|Clamp(Float) (- (Variables|Default|GetSpiritEnergy) 4e+01) 0.0 (Variables|Default|GetMaxSpiritEnergy)))
          (Default|CallOnSpiritCost))))))

(event EventPossessed
  (params (NewController :type Controller%20Object%20Reference))
  (Components|Activation|SetActive (Variables|Default|GetCamera) true false)
  (bind _asplayer_controller (Utilities|Casting|CastToPlayerController NewController))
  (Input|AddMappingContext (PlayerController|LocalPlayerSubsystems|GetEnhancedInputLocalPlayerSubsystem _asplayer_controller) "/Game/PROTOTYE/Input/IMC_MeditateMap.IMC_MeditateMap" 0 "(bIgnoreAllPressedKeysUntilRelease=True,bForceImmediately=False,bNotifyUserSettings=False)"))

(event EventUnpossessed
  (params (OldController :type Controller%20Object%20Reference))
  (Components|Activation|SetActive (Variables|Default|GetCamera) false false)
  (bind _asplayer_controller (Utilities|Casting|CastToPlayerController OldController))
  (Input|RemoveMappingContext (PlayerController|LocalPlayerSubsystems|GetEnhancedInputLocalPlayerSubsystem _asplayer_controller) "/Game/PROTOTYE/Input/IMC_MeditateMap.IMC_MeditateMap" "(bIgnoreAllPressedKeysUntilRelease=True,bForceImmediately=False,bNotifyUserSettings=False)"))

(event EventBeginPlay
  (bind _returnvalue (Actor|GetActorOfClass "/Game/PROTOTYE/Player/BP_Player.BP_Player_C"))
  (Variables|Default|SetPlayer _returnvalue))

(event EventTick
  (params (DeltaSeconds :type Float%20%28single-precision%29))
  (bind _returnvalue (Transformation|GetActorLocation))
  (Utilities|FlowControl|Sequence
    (:then_0
      (if (Class|Pawn|IsControlled)
        (Collision|LineTraceByChannel _returnvalue (+ _returnvalue (* (Math|Vector|GetForwardVector (Variables|Default|GetCamera)) 1e+05)) "TraceTypeQuery1" true 0 "ForDuration" true "(R=1.000000,G=0.000000,B=0.000000,A=1.000000)" "(R=0.000000,G=1.000000,B=0.000000,A=1.000000)" 2.0)
        (else
          (Transformation|SetActorLocation (+ (Transformation|GetActorLocation (Variables|Default|GetPlayer)) (Math|Vector|MakeVector 0.0 0.0 (Variables|Default|GetHeight))) false true))))
    (:then_1
      (Variables|Default|SetSpiritEnergy (Math|Float|Clamp(Float) (+ (Variables|Default|GetSpiritEnergy) (* DeltaSeconds (Variables|Default|GetSpiritRechargeRate))) 0.0 (Variables|Default|GetMaxSpiritEnergy)))
      (Default|CallOnSpiritCost))))

(event Input|KeyboardEvents|1
  (params (Key :type Key%20Structure :default "None"))
  (bind _returnvalue (Transformation|GetActorLocation))
  (:Pressed
    (if (Class|Pawn|IsControlled)
      (bind (_outhit _returnvalue_2) (Collision|LineTraceByChannel _returnvalue (+ _returnvalue (* (Math|Vector|GetForwardVector (Variables|Default|GetCamera)) 1e+05)) "TraceTypeQuery1" true 0 "ForDuration" true "(R=1.000000,G=0.000000,B=0.000000,A=1.000000)" "(R=0.000000,G=1.000000,B=0.000000,A=1.000000)" 2.0))
      (if _returnvalue_2
        (Utilities|IsValid (Variables|Default|GetSpawnedSpirit)
          (:Is%20Not%20Valid
            (bind _returnvalue_3 (Game|SpawnActorfromClass "/Game/PROTOTYE/Spirits/BP_AllySpirit.BP_AllySpirit_C" (Math|Transform|MakeTransform (.Location (Collision|BreakHitResult _outhit))) "AlwaysSpawn" "MultiplyWithRoot" 0 0))
            (Variables|Default|SetSpawnedSpirit _returnvalue_3)
            (Variables|Default|SetSpiritEnergy (Math|Float|Clamp(Float) (- (Variables|Default|GetSpiritEnergy) 4e+01) 0.0 (Variables|Default|GetMaxSpiritEnergy)))
            (Default|CallOnSpiritCost)))))))

(fn ConstructionScript)

(fn QuickSummon
  (bind _player (Variables|Default|GetPlayer))
  (Utilities|IsValid (Variables|Default|GetSpawnedSpirit)
    (:Is%20Valid
      _)
    (:Is%20Not%20Valid
      (if (not (>= (Variables|Default|GetSpiritEnergy) (LocalVariables|GetQuickSummonCost)))
        _
        (else
          (bind _returnvalue (Game|SpawnActorfromClass "/Game/PROTOTYE/Spirits/BP_AllySpirit.BP_AllySpirit_C" (Math|Transform|MakeTransform (+ (Transformation|GetActorLocation _player) (* (Transformation|GetActorRightVector _player) (Math|Float|MakeLiteralFloat -1.5e+02))) (Transformation|GetActorRotation _player)) "AdjustIfPossibleButAlwaysSpawn" "MultiplyWithRoot" 0 0))
          (Variables|Default|SetSpawnedSpirit _returnvalue)
          (Variables|Default|SetSpiritEnergy (Math|Float|Clamp(Float) (- (Variables|Default|GetSpiritEnergy) (LocalVariables|GetQuickSummonCost)) 0.0 (Variables|Default|GetMaxSpiritEnergy)))
          (Default|CallOnSpiritCost)
          (return true)))))
  (return false))

(fn Recall
  (bind _spawnedspirit (Variables|Default|GetSpawnedSpirit))
  (Utilities|IsValid _spawnedspirit
    (:Is%20Valid
      (Actor|DestroyActor _spawnedspirit))))