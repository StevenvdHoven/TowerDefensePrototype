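; Prototype temple actor guarded by ten enemy spirits, taken once all of them are dead or gone.
; On BeginPlay it spawns the spirits at random spawn points.
; Tick draws debug spheres, turns the widget toward the player camera and shows the surviving fraction as progress.
; When none remain alive it calls OnTaken once; IsTaken, despite its name, returns true while spirits still live.
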(event EventBeginPlay
  (CallFunction|SpawnSpirits)
  (bind _aswbp_temple_hud (Utilities|Casting|CastToWBP_TempleHUD (UserInterface|GetUserWidgetObject (Variables|Default|GetWidget))))
  (Variables|Default|SetUI _aswbp_temple_hud))

(event Collision|EventActorBeginOverlap
  (params (OtherActor :type Actor%20Object%20Reference)))

(event EventTick
  (params (DeltaSeconds :type Float%20%28single-precision%29))
  (Utilities|FlowControl|Sequence
    (:then_0
      (CallFunction|DrawDebug))
    (:then_1
      (CallFunction|ManageUIFacing))
    (:then_2
      (CallFunction|UpdateUI))
    (:then_3
      (if (not (Variables|Default|GetAlreadyTaken))
        (if (not (CallFunction|IsTaken))
          (Default|CallOnTaken)
          (Variables|Default|SetAlreadyTaken true))))))

(fn ConstructionScript)

(fn DrawDebug
  (Utilities|FlowControl|Sequence
    (:then_0
      (Rendering|Debug|DrawDebugSphere (Transformation|GetActorLocation) (Variables|TempleSettings|GetRadius) 12 "(R=1.000000,G=0.811638,B=0.000000,A=1.000000)" 0.0 1e+01))
    (:then_1
      (for _array_element (Variables|TempleSettings|GetSpawnPoints)
        (Rendering|Debug|DrawDebugSphere (Transformation|GetActorLocation _array_element) 1e+02 12 "(R=1.000000,G=0.000000,B=0.000000,A=1.000000)" 0.0 5.0)))))

(fn SpawnSpirits
  (while (!= (Utilities|Array|Length (Variables|Default|GetSpawnedSpirits)) 10)
    (bind _returnvalue (Game|SpawnActorfromClass "/Game/PROTOTYE/Spirits/BP_EnemySpirit.BP_EnemySpirit_C" (Transformation|GetActorTransform (.OutItem (Utilities|Array|Random (Variables|TempleSettings|GetSpawnPoints)))) "AlwaysSpawn" "MultiplyWithRoot" self 0))
    (Utilities|IsValid _returnvalue
      (:Is%20Valid
        (Utilities|Array|Add (Variables|Default|GetSpawnedSpirits) _returnvalue))))
  (Variables|Default|SetAlreadySpawnedSpirits true))

(fn ManageUIFacing
  (bind _widget (Variables|Default|GetWidget))
  (Transformation|SetRelativeRotation _widget (Math|Rotator|FindLookatRotation (Transformation|GetWorldLocation _widget) (Camera|GetCameraLocation (Game|GetPlayerCameraManager 0))) false false))

(fn UpdateUI
  (Default|SetProgress (Variables|Default|GetUI) (/ (Math|Conversions|ToFloat(Integer) (CallFunction|GetAliveSpirits)) (Math|Conversions|ToFloat(Integer) (Utilities|Array|Length (Variables|Default|GetSpawnedSpirits))))))

(fn IsTaken
  (return (> (CallFunction|GetAliveSpirits) 0)))

(fn GetAliveSpirits
  (bind _alivespirits (LocalVariables|GetAliveSpirits))
  (if (Variables|Default|GetAlreadySpawnedSpirits)
    (for _array_element (Variables|Default|GetSpawnedSpirits)
      (Utilities|IsValid _array_element
        (:Is%20Valid
          (if (not (Default|IsDead _array_element))
            (Math|Integer|IncrementInt _alivespirits)))))
    (return _alivespirits)
    (else
      (return 10))))