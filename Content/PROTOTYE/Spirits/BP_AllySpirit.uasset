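; Ally spirit character that fights enemy spirits with a melee attack and is destroyed when its health runs out.
; A world-space health widget, tinted blue, rotates every tick to face the player camera and updates whenever TakeDamage reduces the clamped health.
; Attack plays a fist montage and immediately runs a sphere overlap in front of the spirit, dealing fixed damage to any BP_EnemySpirit found.
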(event EventBeginPlay
  (bind _aswbp_spirit_health_display (Utilities|Casting|CastToWBP_SpiritHealthDisplay (UserInterface|GetWidget (Variables|Default|GetWidget))))
  (bind _output_get (Variables|Default|SetUI _aswbp_spirit_health_display))
  (Default|SetHealthBarColor _output_get (Math|Conversions|ToColor(LinearColor) (Class|KismetMathLibrary|LinearColorBlue))))

(event EventTick
  (params (DeltaSeconds :type Float%20%28single-precision%29))
  (bind _widget (Variables|Default|GetWidget))
  (Transformation|SetWorldRotation _widget (Math|Rotator|FindLookatRotation (Transformation|GetWorldLocation _widget) (Camera|GetCameraLocation (Game|GetPlayerCameraManager 0))) false false))

(event EventTakeDamage
  (params (Damage :type Integer))
  (bind _output_get (Variables|Default|SetHealth (Math|Integer|Clamp(Integer) (- (Variables|Default|GetHealth) Damage) 0 100)))
  (Utilities|FlowControl|Sequence
    (:then_0
      (Default|SetHealthPercent (Variables|Default|GetUI) (/ (Math|Conversions|ToFloat(Integer) (Variables|Default|GetHealth)) 1e+02)))
    (:then_1
      (if (<= _output_get 0)
        (Actor|DestroyActor)))))

(fn ConstructionScript)

(fn Attack
  (Animation|PlayAnimMontage "/Game/FlexibleCombatSystem/Montages/M_Fists_AttackA.M_Fists_AttackA" 1.0 "None")
  (bind _outactors (Collision|SphereOverlapActors (+ (Transformation|GetActorLocation) (* (Transformation|GetActorForwardVector) (Math|Float|MakeLiteralFloat 1.5e+02))) 1e+02 (Utilities|Array|MakeArray "ObjectTypeQuery1" "ObjectTypeQuery2" "ObjectTypeQuery3" "ObjectTypeQuery4" "ObjectTypeQuery5" "ObjectTypeQuery6") "/Script/Engine.Character" (Utilities|Array|MakeArray self)))
  (for _array_element _outactors
    (bind _asbp_enemy_spirit (Utilities|Casting|CastToBP_EnemySpirit _array_element))
    (Default|TakeDamage _asbp_enemy_spirit 20)))