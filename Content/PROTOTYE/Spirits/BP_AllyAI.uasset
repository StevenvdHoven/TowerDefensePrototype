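; BP_AllyAI is the AI controller for allied spirits, driving them with the BT_AllySpirit behavior tree and BB_AllySpirit blackboard.
; On BeginPlay it stores the player actor in the blackboard and starts the tree.
; Perception updates write a living enemy spirit to the SeenEnemy key only when that key is empty or its current enemy is dead, so the target stays locked until it dies.
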(event OnTargetPerceptionUpdated(AIPerception)
  (params (Actor :type Actor%20Object%20Reference) (Stimulus :type AI%20Stimulus%20Structure))
  (bind _returnvalue (AI|GetBlackboard 0))
  (bind _returnvalue_2 (Utilities|Name|MakeLiteralName "SeenEnemy"))
  (bind _returnvalue_3 (AI|Components|Blackboard|GetValueasObject _returnvalue _returnvalue_2))
  (bind _asbp_enemy_spirit (Utilities|Casting|CastToBP_EnemySpirit Actor))
  (if (not (Default|IsDead _asbp_enemy_spirit))
    (Utilities|IsValid _returnvalue_3
      (:Is%20Valid
        (bind _asbp_enemy_spirit_2 (Utilities|Casting|CastToBP_EnemySpirit _returnvalue_3))
        (if (Default|IsDead _asbp_enemy_spirit_2)
          (AI|Components|Blackboard|SetValueasObject _returnvalue _returnvalue_2 _asbp_enemy_spirit :!label _label)))
      (:Is%20Not%20Valid
        (goto _label)))))

(event EventBeginPlay
  (Class|AIController|UseBlackboard "/Game/PROTOTYE/Spirits/BB_AllySpirit.BB_AllySpirit")
  (bind _returnvalue (Actor|GetActorOfClass "/Game/PROTOTYE/Player/BP_Player.BP_Player_C"))
  (AI|Components|Blackboard|SetValueasObject (AI|GetBlackboard 0) (Utilities|Name|MakeLiteralName "Player") _returnvalue)
  (AI|RunBehaviorTree "/Game/PROTOTYE/Spirits/BT_AllySpirit.BT_AllySpirit"))

(fn ConstructionScript)