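; BP_EnemySpirit is a prototype enemy spirit with a health pool that can be damaged until it dies.
; Its TakeDamage event ignores hits once dead, otherwise subtracts clamped damage from Health and prints the amount on screen for debugging.
; When IsDead reports Health at zero or below, the actor is hidden and collision on its capsule and cylinder is disabled, rather than being destroyed.
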(event EventTakeDamage
  (params (Damage :type Integer))
  (if (not (CallFunction|IsDead))
    (Utilities|FlowControl|Sequence
      (:then_0
        (Variables|Default|SetHealth (Math|Integer|Clamp(Integer) (- (Variables|Default|GetHealth) Damage) 0 (Variables|Default|GetHealth))))
      (:then_1
        (Development|PrintString (Utilities|String|Append (Utilities|String|MakeLiteralString "Damage: ") (Utilities|String|ToString(Integer) Damage)) true false "(R=1.000000,G=0.059065,B=0.000000,A=1.000000)"))
      (:then_2
        (if (CallFunction|IsDead)
          (Rendering|SetActorHiddenInGame true)
          (Collision|SetCollisionEnabled (Variables|Collision|GetCapsuleComponent) "NoCollision"))))))

(fn ConstructionScript)

(fn IsDead
  (return (<= (Variables|Default|GetHealth) 0)))