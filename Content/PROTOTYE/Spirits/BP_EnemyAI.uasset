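; BP_EnemyAI is the AI controller logic for enemy spirits, driven by behavior tree BT_EnemySpirit and blackboard BB_EnemySpirit.
; On BeginPlay it stores its own location as StartPosition, runs the tree, and binds to OnDead if its owner is a BP_EnemySpirit.
; AI perception updates involving BP_Player write SeenActor without checking sense success or clearing it.
; The death event stops the brain logic.
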(event OnTargetPerceptionUpdated(AIPerception)
  (params (Actor :type Actor%20Object%20Reference) (Stimulus :type AI%20Stimulus%20Structure))
  (bind _asbp_player (Utilities|Casting|CastToBP_Player Actor))
  (AI|Components|Blackboard|SetValueasObject (AI|GetBlackboard 0) (Utilities|Name|MakeLiteralName "SeenActor") _asbp_player))

(event Custom|OnDead_Event
  (AI|Logic|StopLogic (Variables|Default|GetBrainComponent) ""))

(event EventBeginPlay
  (Utilities|FlowControl|Sequence
    (:then_0
      (bind _blackboardcomponent (Class|AIController|UseBlackboard "/Game/PROTOTYE/Spirits/BB_EnemySpirit.BB_EnemySpirit"))
      (AI|Components|Blackboard|SetValueasVector _blackboardcomponent (Utilities|Name|MakeLiteralName "StartPosition") (Transformation|GetActorLocation))
      (AI|RunBehaviorTree "/Game/PROTOTYE/Spirits/BT_EnemySpirit.BT_EnemySpirit"))
    (:then_1
      (bind _asbp_enemy_spirit (Utilities|Casting|CastToBP_EnemySpirit (Components|GetOwner)))
      (EventDispatchers|AssignOnDead _asbp_enemy_spirit (delegate Custom|OnDead_Event)))))

(fn ConstructionScript)