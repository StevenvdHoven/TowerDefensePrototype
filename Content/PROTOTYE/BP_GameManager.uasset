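; BP_GameManager tracks the level's BP_Temple actors and shows temple capture progress on the HUD.
; On BeginPlay it gathers all temples, binds their OnTaken events, and creates WBP_HUD with the temple total.
; Each OnTaken event refreshes the HUD through UpdateUI.
; The count passed as captured temples increments for temples where IsTaken is false, despite the function's name.
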(event Custom|OnTaken
  (CallFunction|UpdateUI))

(event EventBeginPlay
  (Utilities|FlowControl|Sequence
    (:then_0
      (bind _outactors (Actor|GetAllActorsOfClass "/Game/PROTOTYE/Temples/BP_Temple.BP_Temple_C"))
      (bind _output_get (Variables|Default|SetTemples _outactors))
      (for _array_element _output_get
        (EventDispatchers|BindEventtoOnTaken _array_element (delegate Custom|OnTaken))))
    (:then_1
      (bind _returnvalue (UserInterface|CreateWidget "/Game/PROTOTYE/WBP_HUD.WBP_HUD_C"))
      (bind _output_get_2 (Variables|Default|SetUI _returnvalue))
      (Variables|/Game/PROTOTYE/WBP_HUD.WBP_HUD_C|SetMaxTemples _output_get_2 (Utilities|Array|Length (Variables|Default|GetTemples)))
      (UserInterface|Viewport|AddtoViewport _output_get_2 0))
    (:then_2
      (CallFunction|UpdateUI))))

(fn ConstructionScript)

(fn AddTemple
  (params (temple :type BP%20Temple%20Object%20Reference))
  (Utilities|Array|AddUnique (Variables|Default|GetTemples) temple))

(fn UpdateUI
  (Default|UpdateTemples (Variables|Default|GetUI) (CallFunction|GetCapturedTempels)))

(fn GetCapturedTempels
  (bind _capturedtemples (LocalVariables|GetcapturedTemples))
  (for _array_element (Variables|Default|GetTemples)
    (if (not (Default|IsTaken _array_element))
      (Math|Integer|IncrementInt _capturedtemples)))
  (return _capturedtemples))